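; BP_Field is the MashRunner stage, built procedurally from StagePartCount and StageLength in the construction script.
; It tiles SPR_Field Paper2D sprite components along X, one per stage part.
; InitBox stretches BoxTop and BoxBottom to span and center on the whole strip, while GoalTop and GoalBottom shift to the last part.
; The event graph holds no active logic.
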(fn `InitBox`
  (params (Box :type "BoxComponent Object Reference"))
  (bind (_boxextent_x _boxextent_y _boxextent_z) (`KismetMathLibrary.BreakVector` (`BoxComponent.BoxExtent` (`local.Box`))))
  (bind (_relativelocation_x _relativelocation_y _relativelocation_z) (`KismetMathLibrary.BreakVector` (`SceneComponent.RelativeLocation` (`local.Box`))))
  (`BoxComponent.SetBoxExtent` (`local.Box`) (`KismetMathLibrary.MakeVector` (`KismetMathLibrary.Conv_IntToDouble` (* (/ (`self.StageLength`) 2) (`self.StagePartCount`))) _boxextent_y _boxextent_z) true)
  (`SceneComponent.K2_SetRelativeLocation` (`local.Box`) (`KismetMathLibrary.MakeVector` (`KismetMathLibrary.Conv_IntToDouble` (- (/ (* (`self.StageLength`) (`self.StagePartCount`)) 2) (/ (`self.StageLength`) 2))) _relativelocation_y _relativelocation_z) false false))

(fn `UserConstructionScript`
  (bind (_relativelocation_x _relativelocation_y _relativelocation_z) (`KismetMathLibrary.BreakVector` (`SceneComponent.RelativeLocation` (`self.GoalBottom`))))
  (bind (_relativelocation_x_2 _relativelocation_y_2 _relativelocation_z_2) (`KismetMathLibrary.BreakVector` (`SceneComponent.RelativeLocation` (`self.GoalTop`))))
  (for _index (range (`self.StagePartCount`))
    (bind _returnvalue (`AddComponent|NODE_AddPaperSpriteComponent-0` :`RelativeTransform` (`KismetMathLibrary.MakeTransform` (`KismetMathLibrary.MakeVector` (`KismetMathLibrary.Conv_IntToDouble` (* _index (`self.StageLength`)))))))
    (`PaperSpriteComponent.SetSprite` _returnvalue "/Game/MashRunner/Art/Background/SPR_Field.SPR_Field"))
  (`self.InitBox` (`self.BoxTop`))
  (`self.InitBox` (`self.BoxBottom`))
  (`SceneComponent.K2_SetRelativeLocation` (`self.GoalBottom`) (`KismetMathLibrary.MakeVector` (+ (* (- (`self.StagePartCount`) 1) (`self.StageLength`)) _relativelocation_x) _relativelocation_y _relativelocation_z) false false)
  (`SceneComponent.K2_SetRelativeLocation` (`self.GoalTop`) (`KismetMathLibrary.MakeVector` (+ (* (- (`self.StagePartCount`) 1) (`self.StageLength`)) _relativelocation_x_2) _relativelocation_y_2 _relativelocation_z_2) false false))